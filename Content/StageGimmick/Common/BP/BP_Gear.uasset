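; BP_Gear is a stage gimmick gear that shuttles back and forth between a start and end position while spinning.
; The Moving timeline starts on BeginPlay and lerps the gear mesh's relative location between the two points.
; When the timeline finishes, its direction selects reverse or forward playback, looping the motion indefinitely.
; Tick adds a fixed local rotation every frame, so spin speed depends on frame rate.
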(event `self.ReceiveBeginPlay`
  ; Start地点とEnd地点の2点間を往復移動する(現在の片道移動時間は3秒)
  (bind (_direction _movingrate) (`Timeline|Moving` :`NewTime` 0.0 :!label _label) ; ２点間移動TimeLine
    (:`Update`
      (`SceneComponent.K2_SetRelativeLocation` (`self.SM_Gear`) (`KismetMathLibrary.VLerp` (`self.StartPosition`) (`self.EndPosition`) _movingrate) false false) ; Objectの位置移動
    )
    (:`Finished`
      (switch `ETimelineDirection` _direction ; 終了時の準再生・逆再生の切替判定
        (:`Forward`
          (`self.PlayBackward`) ; TimeLine終了時に逆再生する
        )
        (:`Backward`
          (`self.PlayFoward`) ; TimeLine逆再生終了時準再生する
        )))))

(event `PlayBackward`
  ; Start地点とEnd地点の2点間を往復移動する(現在の片道移動時間は3秒)
  (goto _label :!via `Reverse`))

(event `PlayFoward`
  ; Start地点とEnd地点の2点間を往復移動する(現在の片道移動時間は3秒)
  (goto _label))

(event `self.ReceiveTick`
  (params (DeltaSeconds :type "Float (single-precision)"))
  ; 歯車自身の回転処理
  (`SceneComponent.K2_AddLocalRotation` (`self.SM_Gear`) (struct :`Yaw` 1.0) false false))

(fn `UserConstructionScript`)