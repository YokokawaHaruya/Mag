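; Magnetic actor prototype that decides how it should attract or repel other BP_MagneticActor objects entering its field.
; The construction script sizes the field sphere from radius variables, and BeginPlay applies the mobility setting to the mesh.
; On overlap, the other actor's pole type, mobility and polarity match select a Japanese debug message describing the interaction.
; No force is applied, as the radial impulse nodes are unwired.
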(event `self.ReceiveBeginPlay`
  (`SceneComponent.SetMobility` (`self.Mesh`) (`self.Mobility`)))

(event `self.MagneticFieldCollision.OnComponentBeginOverlap`
  (params (OverlappedComponent :type "PrimitiveComponent Object Reference") (OtherActor :type "Actor Object Reference") (OtherComp :type "PrimitiveComponent Object Reference") (OtherBodyIndex :type Integer) (bFromSweep :type Boolean) (SweepResult :type "HitResult Structure (by ref)"))
  (bind _returnvalue (== (`KismetMathLibrary.Conv_ByteToInt` (`self.OtherPolaryType`)) (`KismetMathLibrary.Conv_ByteToInt` (`self.PolaryType`))))
  (bind _asbp_magnetic_actor (cast `/Game/001_Mag/020_BP/BP_MagneticActor` OtherActor))
  (bind _output_get (set `self.OtherPolaryType` (`/Game/001_Mag/020_BP/BP_MagneticActorCopy.PolaryType` _asbp_magnetic_actor)))
  (switch `/Game/001_Mag/020_BP/En_PolaryType` _output_get
    (:`NewEnumerator0`
      (bind _mobility (`/Game/001_Mag/020_BP/BP_MagneticActorCopy.Mobility` _asbp_magnetic_actor))
      (switch `EComponentMobility` _mobility
        (:`Static`
          (`KismetSystemLibrary.PrintText` "引っ張られる"))
        (:`Movable`
          (`KismetSystemLibrary.PrintText` "引っ張る"))))
    (:`NewEnumerator1`
      (switch `EComponentMobility` _mobility :!label _label
        (:`Static`
          (if _returnvalue
            (`KismetSystemLibrary.PrintText` "突き放される")
            (else
              (`KismetSystemLibrary.PrintText` "引き寄せられる"))))
        (:`Movable`
          (if _returnvalue
            (`KismetSystemLibrary.PrintText` "突き放しあう")
            (else
              (`KismetSystemLibrary.PrintText` "引き寄せあう"))))))
    (:`NewEnumerator2`
      (goto _label))))

(fn `UserConstructionScript`
  (`SphereComponent.SetSphereRadius` (`self.MagneticFieldCollision`) (* (`self.CollisionRadius`) (`self.DefaultRadius`)) true))

(fn `新規関数`)