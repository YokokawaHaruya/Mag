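; BP_MagneticActor is a work-in-progress magnet actor with configurable mobility and a sphere magnetic field.
; The construction script sizes the field and sets the mesh's collision channel.
; Overlapping another BP_MagneticActor starts a looping timer that fires a radial impulse while SuctionCount, which is never incremented, stays below two.
; Polarity-based attract/repel branches are disconnected debug prints, and the MagneticRepulsive and MagneticAttraction functions are stubs.
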(event `self.ReceiveBeginPlay`
  (`SceneComponent.SetMobility` (`self.MagnetMesh`) (`self.Mobility`)))

(event `self.MagneticFieldCollision.OnComponentBeginOverlap`
  (params (OverlappedComponent :type "PrimitiveComponent Object Reference") (OtherActor :type "Actor Object Reference") (OtherComp :type "PrimitiveComponent Object Reference") (OtherBodyIndex :type Integer) (bFromSweep :type Boolean) (SweepResult :type "HitResult Structure (by ref)"))
  (`KismetSystemLibrary.PrintString` (`KismetSystemLibrary.GetDisplayName` OtherComp) true true (struct :`G` 0.66 :`B` 1.0 :`A` 1.0) 10.0)
  (`KismetSystemLibrary.PrintString` (`KismetSystemLibrary.GetDisplayName` OverlappedComponent) true true (struct :`G` 0.66 :`B` 1.0 :`A` 1.0) 10.0)
  (bind _asbp_magnetic_actor (cast `/Game/001_Mag/020_BP/BP_MagneticActor` OtherActor)
    (:`then`
      (`|ExecutionSequence`
        (:`then_0`
          (`KismetSystemLibrary.PrintString` "cast true"))
        (:`then_1`
          (bind _returnvalue (`KismetSystemLibrary.K2_SetTimer` null "Ev_Suction" 0.1 true))
          (set `self.SuctionTimer` _returnvalue))))
    (:`CastFailed`
      (`KismetSystemLibrary.PrintString` "castfailed"))))

(event `Ev_Suction`
  (bind _magneticforce (`self.MagneticForce`))
  (bind _output_get (set `self.SuctionCount` (`self.SuctionCount`)))
  (if (< _output_get 2.0)
    (`KismetSystemLibrary.PrintString` (`KismetSystemLibrary.GetDisplayName` _magneticforce))
    (set `RadialForceComponent.Radius` (`RadialForceComponent.Radius` _magneticforce) _magneticforce)
    (set `RadialForceComponent.ImpulseStrength` 30000.0 _magneticforce)
    (`RadialForceComponent.FireImpulse` (`self.MagneticForce`))
    (else
      (`KismetSystemLibrary.K2_ClearAndInvalidateTimerHandle` (`self.SuctionTimer`))
      (set `self.SuctionCount` 0.0))))

(event `self.MagnetMesh.OnComponentHit`
  (params (HitComponent :type "PrimitiveComponent Object Reference") (OtherActor :type "Actor Object Reference") (OtherComp :type "PrimitiveComponent Object Reference") (NormalImpulse :type "Vector Structure") (Hit :type "HitResult Structure (by ref)")))

(event `self.MagnetMesh.OnComponentEndOverlap`
  (params (OverlappedComponent :type "PrimitiveComponent Object Reference") (OtherActor :type "Actor Object Reference") (OtherComp :type "PrimitiveComponent Object Reference") (OtherBodyIndex :type Integer))
  (cast `/Game/001_Mag/020_BP/BP_MagneticActor` OtherActor)
  (set `self.IsCollision` false)
  (`KismetSystemLibrary.PrintString` "hit end"))

(fn `MagneticAttraction`)

(fn `MagneticRepulsive`
  (returns (NewParam :type Boolean))
  (return false))

(fn `UserConstructionScript`
  (`SphereComponent.SetSphereRadius` (`self.MagneticFieldCollision`) (* (`self.SphereRadius`) (`self.DefaultRadius`)) true)
  (`PrimitiveComponent.SetCollisionObjectType` (`self.MagnetMesh`) "ECC_GameTraceChannel5"))