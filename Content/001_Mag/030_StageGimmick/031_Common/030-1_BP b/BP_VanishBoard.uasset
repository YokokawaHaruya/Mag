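; BP_VanishBoard is a stage-gimmick floor board that vanishes a set time after the player steps on it.
; Box overlap with the player pawn calls VanishBoard, which waits for Duration, destroys the actor, then sets IsVanished.
; Tick spawns a new BP_VanishBoard at SpawnTransform while IsVanished is true, though that flag is only set after DestroyActor.
; A hide-in-game call is left unconnected.
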(event `self.ReceiveBeginPlay`)

(event `self.ReceiveTick`
  (params (DeltaSeconds :type "Float (single-precision)"))
  (if (`self.isVanished`)
    (`|SpawnActorFromClass` "BP_VanishBoard_C" (`self.Spawn Transform`) "Undefined" "MultiplyWithRoot" null null)))

(event `self.Box.OnComponentBeginOverlap`
  (params (OverlappedComponent :type "PrimitiveComponent Object Reference") (OtherActor :type "Actor Object Reference") (OtherComp :type "PrimitiveComponent Object Reference") (OtherBodyIndex :type Integer) (bFromSweep :type Boolean) (SweepResult :type "HitResult Structure (by ref)"))
  ; 床にPlayerが乗ると一定時間後に消滅する
  (if (== OtherActor (`GameplayStatics.GetPlayerPawn` 0))
    (`self.VanishBoard`)
    (if true
      _)))

(event `VanishBoard`
  (`KismetSystemLibrary.Delay` (`self.Duration`)) ; 処理動作を一定時間停止
  (`self.K2_DestroyActor`)
  (set `self.isVanished` true))

(fn `UserConstructionScript`)