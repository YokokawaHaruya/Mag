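; BP_SpikeCube is a death-gimmick trap whose spiked cube lunges when the player pawn enters its trigger and then retracts.
; The trigger overlap sets a flag that Tick reads to play or reverse the Moving timeline, with speed driven by GimmickSpeedRate.
; The timeline slides the cube mesh along local Y and clears the flag on finishing.
; A separate damage collision applies heavy fixed damage to the player on overlap.
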(event `self.ReceiveTick`
  (params (DeltaSeconds :type "Float (single-precision)"))
  (`TimelineComponent.SetPlayRate` (`self.Moving`) (`self.GimmickSpeedRate`))
  (if (`self.Flag`)
    (bind (_direction _spilecubeposition) (`Timeline|Moving` :!label _label)
      (:`Update`
        (`SceneComponent.K2_SetRelativeLocation` (`self.SM_SpikeCube`) (`KismetMathLibrary.MakeVector` 0.0 _spilecubeposition) false false))
      (:`Finished`
        (set `self.Flag` false)))
    (else
      (goto _label :!via `Reverse`))))

(event `self.TrapCollision.OnComponentBeginOverlap`
  (params (OverlappedComponent :type "PrimitiveComponent Object Reference") (OtherActor :type "Actor Object Reference") (OtherComp :type "PrimitiveComponent Object Reference") (OtherBodyIndex :type Integer) (bFromSweep :type Boolean) (SweepResult :type "HitResult Structure (by ref)"))
  (if (== OtherActor (`GameplayStatics.GetPlayerPawn` 0))
    (set `self.Flag` true)))

(event `self.DamgeCollision.OnComponentBeginOverlap`
  (params (OverlappedComponent :type "PrimitiveComponent Object Reference") (OtherActor :type "Actor Object Reference") (OtherComp :type "PrimitiveComponent Object Reference") (OtherBodyIndex :type Integer) (bFromSweep :type Boolean) (SweepResult :type "HitResult Structure (by ref)"))
  (bind _returnvalue (`GameplayStatics.GetPlayerPawn` 0))
  (if (== OtherActor _returnvalue)
    (`GameplayStatics.ApplyDamage` _returnvalue 100.0)))

(fn `UserConstructionScript`)