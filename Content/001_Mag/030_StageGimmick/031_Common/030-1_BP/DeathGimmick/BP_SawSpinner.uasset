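; BP_SawSpinner is a death gimmick: a spinning saw blade that shuttles along a bar and damages the player on contact.
; A Moving timeline, with adjustable play speed, drives the blade's relative Y from the bar's world Y scale and reverses each time it finishes.
; Tick rolls the blade at a set speed, while the saw collision's begin-overlap applies fixed damage only to the player pawn.
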(event `self.ReceiveBeginPlay`
  (bind (_returnvalue_x _returnvalue_y) (`KismetMathLibrary.BreakVector` (`SceneComponent.K2_GetComponentScale` (`self.Bar`))))
  ; 回転のこぎりBar上の始点・終点間の移動処理
  (`TimelineComponent.SetPlayRate` (`self.Moving`) (`self.PlaySpeed`)) ; 回転のこぎり移動速度倍率の初期化
  (bind (_direction _movingrate) (`Timeline|Moving` :!label _label)
    (:`Update`
      (`SceneComponent.K2_SetRelativeLocation` (`self.SawSpinner`) (`KismetMathLibrary.MakeVector` 0.0 (* _movingrate _returnvalue_y)) false false) ; のこぎり刃の位置を更新する
    )
    (:`Finished`
      (switch `ETimelineDirection` _direction ; 終了時の準再生・逆再生の切替判定
        (:`Forward`
          (`self.Play Backward`) ; 逆再生する
        )
        (:`Backward`
          (`self.Play Fowrd`) ; 標準再生する
        )))))

(event `Play Fowrd`
  ; 回転のこぎりBar上の始点・終点間の移動処理
  (goto _label))

(event `Play Backward`
  ; 回転のこぎりBar上の始点・終点間の移動処理
  (goto _label :!via `Reverse`))

(event `self.ReceiveTick`
  (params (DeltaSeconds :type "Float (single-precision)"))
  ; のこぎり刃自身の回転処理
  (`SceneComponent.K2_AddLocalRotation` (`self.SawSpinner`) (`KismetMathLibrary.MakeRotator` (`self.SawRotationSpeed`)) false false) ; のこぎり刃の回転処理
)

(event `self.SawCollision.OnComponentBeginOverlap`
  (params (OverlappedComponent :type "PrimitiveComponent Object Reference") (OtherActor :type "Actor Object Reference") (OtherComp :type "PrimitiveComponent Object Reference") (OtherBodyIndex :type Integer) (bFromSweep :type Boolean) (SweepResult :type "HitResult Structure (by ref)"))
  (bind _returnvalue (`GameplayStatics.GetPlayerPawn` 0))
  ; のこぎり刃当たり判定処理
  (if (== OtherActor _returnvalue)
    (`GameplayStatics.ApplyDamage` _returnvalue 100.0) ; Playerにダメージを与える
  ))

(fn `UserConstructionScript`)