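; BP_RotationSpike is a stage death gimmick: a rotating spike that damages the player on contact.
; Tick spins the SMRotationSpike component in yaw by a negated RotationSpeed for counterclockwise motion, applied per frame without delta-time scaling.
; Two collision components each check on begin overlap for player pawn 0 and apply a fixed, heavy damage hit.
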(event `self.ReceiveTick`
  (params (DeltaSeconds :type "Float (single-precision)"))
  ; Spike自身の回転処理
  (`SceneComponent.K2_AddLocalRotation` (`self.SM_Rotation_Spike`) (`KismetMathLibrary.MakeRotator` 0.0 0.0 (* (`self.RotationSpeed`) -1.0)) false false))

(event `self.SpileCollison_1.OnComponentBeginOverlap`
  (params (OverlappedComponent :type "PrimitiveComponent Object Reference") (OtherActor :type "Actor Object Reference") (OtherComp :type "PrimitiveComponent Object Reference") (OtherBodyIndex :type Integer) (bFromSweep :type Boolean) (SweepResult :type "HitResult Structure (by ref)"))
  (bind _returnvalue (`GameplayStatics.GetPlayerPawn` 0))
  ; Spike当たり判定処理
  (if (== OtherActor _returnvalue)
    (`GameplayStatics.ApplyDamage` _returnvalue 100.0) ; Damage処理
  ))

(event `self.SpileCollison_2.OnComponentBeginOverlap`
  (params (OverlappedComponent :type "PrimitiveComponent Object Reference") (OtherActor :type "Actor Object Reference") (OtherComp :type "PrimitiveComponent Object Reference") (OtherBodyIndex :type Integer) (bFromSweep :type Boolean) (SweepResult :type "HitResult Structure (by ref)"))
  (bind _returnvalue (`GameplayStatics.GetPlayerPawn` 0))
  ; Spike当たり判定処理
  (if (== OtherActor _returnvalue)
    (`GameplayStatics.ApplyDamage` _returnvalue 100.0)))

(fn `UserConstructionScript`)