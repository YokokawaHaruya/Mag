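; Needle board death gimmick that raises and lowers spikes and kills the player on contact.
; If IsPlay is set at BeginPlay, the Moving timeline drives the Needle's relative Z at a PlaySpeedRate-scaled speed.
; On finish, the timeline flips between Play and Reverse for an endless ping-pong.
; NeedleCollision overlap with player pawn 0 applies fixed damage intended as an instant kill.
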(event `self.ReceiveBeginPlay`
  ; Needleギミックの再生処理
  (`TimelineComponent.SetPlayRate` (`self.Moving`) (`self.PlaySpeedRate`)) ; 回転のこぎり移動速度倍率の初期化
  (if (`self.IsPlay`)
    (bind (_direction _needleposition_z_) (`Timeline|Moving` :!label _label)
      (:`Update`
        (`SceneComponent.K2_SetRelativeLocation` (`self.Needle`) (`KismetMathLibrary.MakeVector` 0.0 0.0 _needleposition_z_) false false) ; Needleと当たり判定のＺ位置を更新する
      )
      (:`Finished`
        (switch `ETimelineDirection` _direction ; 終了時の準再生・逆再生の切替判定
          (:`Forward`
            (`self.Play Backward`) ; 逆再生する
          )
          (:`Backward`
            (`self.Play Fowrd`) ; 標準再生する
          ))))))

(event `Play Fowrd`
  ; Needleギミックの再生処理
  (goto _label))

(event `Play Backward`
  ; Needleギミックの再生処理
  (goto _label :!via `Reverse`))

(event `self.NeedleCollision.OnComponentBeginOverlap`
  (params (OverlappedComponent :type "PrimitiveComponent Object Reference") (OtherActor :type "Actor Object Reference") (OtherComp :type "PrimitiveComponent Object Reference") (OtherBodyIndex :type Integer) (bFromSweep :type Boolean) (SweepResult :type "HitResult Structure (by ref)"))
  (bind _returnvalue (`GameplayStatics.GetPlayerPawn` 0))
  ; 針に当たったときの当たり判定処理
  (if (== OtherActor _returnvalue)
    (`GameplayStatics.ApplyDamage` _returnvalue 100.0) ; Playerにダメージ(即死)を与える
  ))

(fn `UserConstructionScript`)